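; Test Blueprint for a TPS inventory item, used to pass data into the item and check it.
; SetTestData prints its int, float, string, bool and vector arguments to verify they arrive.
; SetInventoryData stores the inventory data and a test color, then calls Init.
; GenerateColor returns that stored color, and the default BeginPlay, overlap and Tick events are unused.
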(event Custom|SetTestData
  (params (Int :type Integer) (Float :type Float%20%28single-precision%29) (Str :type String) (Bool :type Boolean) (Vec :type Vector))
  (Development|PrintString (Utilities|String|ToString(Integer) Int))
  (Development|PrintString (Utilities|String|ToString(Float) Float))
  (Development|PrintString Str)
  (Development|PrintString (Utilities|String|ToString(Boolean) Bool))
  (Development|PrintString (Utilities|String|ToString(Vector) Vec)))

(event Custom|SetInventoryData
  (params (InvData :type Inventory%20Data%20Structure) (Color :type Linear%20Color%20Structure))
  (Variables|Default|SetInventoryData InvData)
  (Variables|Default|SetTestColor Color)
  (CallFunction|Init))

(event EventBeginPlay
  (|CallParentFunction) ; This node is disabled and will not be called.\nDrag off pins to build functionality.
)

(event Collision|EventActorBeginOverlap
  (params (OtherActor :type Actor%20Object%20Reference))
  (|CallParentFunction OtherActor) ; This node is disabled and will not be called.\nDrag off pins to build functionality.
)

(event EventTick
  (params (DeltaSeconds :type Float%20%28single-precision%29))
  (|CallParentFunction DeltaSeconds) ; This node is disabled and will not be called.\nDrag off pins to build functionality.
)

(fn ConstructionScript
  (|CallParentFunction))

(fn GenerateColor
  (return (Variables|Default|GetTestColor)))